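; BasicEnemy is an AI-controlled enemy that patrols a looping route of waypoint actors.
; On BeginPlay it issues an AI MoveTo toward the waypoint at the current index.
; When the move finishes, it advances the index with a modulo wrap and calls the WaypointReached event, which starts the next move and keeps the patrol running indefinitely.
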(event Custom|WaypointReached
  (AI|AIMoveTo (AI|GetAIController self) "0, 0, 0" (Utilities|Array|Get(acopy) (Variables|Default|GetWaypoints) (Variables|Default|GetWaypointToReference)) -1.0 "Default" "Default" true true
    (:OnMoveFinished
      (Variables|Default|SetWaypointToReference (Math|Integer|%(Integer) (+ (Variables|Default|GetWaypointToReference) 1) (Utilities|Array|Length (Variables|Default|GetWaypoints))))
      (CallFunction|WaypointReached))))

(event EventBeginPlay
  (AI|AIMoveTo (AI|GetAIController self) "0, 0, 0" (Utilities|Array|Get(acopy) (Variables|Default|GetWaypoints) (Variables|Default|GetWaypointToReference)) -1.0 "Default" "Default" true true
    (:OnMoveFinished
      (Variables|Default|SetWaypointToReference (Math|Integer|%(Integer) (+ (Variables|Default|GetWaypointToReference) 1) (Utilities|Array|Length (Variables|Default|GetWaypoints))))
      (CallFunction|WaypointReached))))

(fn ConstructionScript)